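; Water Form spell actor that temporarily boosts the player's magic power.
; On BeginPlay it loads mana cost, damage modifier and cooldown from the Spells data table, deducts mana and scales cooldown by the player's cooldown reduction.
; It multiplies MagicPower by the damage modifier, then divides it back after a five-second delay.
; The computed damage, cooldown and saved starting magic power are not used further in this graph.
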(event `self.ReceiveBeginPlay`
  (bind _player (`self.Player`))
  (bind _cooldown_time (`self.Cooldown Time`))
  (`|ExecutionSequence`
    (:`then_0`
      (bind _returnvalue (`|GetDataTableRow` "/Game/Blueprints/Spells_-_Spells.Spells_-_Spells" "WaterForm_C")
        (:`then`
          (set `self.Mana Cost` (`.ManaCost_7_C903C12F4449ABCC6E8F80B36C51241A` (break `/Game/Blueprints/SpellsData` _returnvalue)))
          (set `self.Damage Modifier` (`.SpellDamage_3_53CF477246276293E4E13B8EC3A5A41E` (break `/Game/Blueprints/SpellsData` _returnvalue)))
          (set `self.Cooldown Time` (`.Cooldown_20_4E963C174A27AC4E215781B8BC1AD210` (break `/Game/Blueprints/SpellsData` _returnvalue))))))
    (:`then_1`
      (bind _asthird_person_character (cast `/Game/Blueprints/ThirdPersonBP/Blueprints/ThirdPersonCharacter` (`GameplayStatics.GetPlayerCharacter` 0)))
      (set `self.Player` _asthird_person_character)
      (set `/Game/Blueprints/ThirdPersonBP/Blueprints/ThirdPersonCharacter.Mana` (- (`/Game/Blueprints/ThirdPersonBP/Blueprints/ThirdPersonCharacter.Mana` _asthird_person_character) (`self.Mana Cost`)) _asthird_person_character)
      (set `self.Damage` (* (`/Game/Blueprints/ThirdPersonBP/Blueprints/ThirdPersonCharacter.Magic Power` _asthird_person_character) (`self.Damage Modifier`)))
      (set `self.Cooldown Time` (- _cooldown_time (* _cooldown_time (/ (`/Game/Blueprints/ThirdPersonBP/Blueprints/ThirdPersonCharacter.Cooldown Reduction` _asthird_person_character) 100.0)))))
    (:`then_2`
      (set `self.Player Beginning Magic Power` (`/Game/Blueprints/ThirdPersonBP/Blueprints/ThirdPersonCharacter.Magic Power` (`self.Player`))))
    (:`then_3`
      (bind _output_get (set `/Game/Blueprints/ThirdPersonBP/Blueprints/ThirdPersonCharacter.Magic Power` (* (`/Game/Blueprints/ThirdPersonBP/Blueprints/ThirdPersonCharacter.Magic Power` _player) (`self.Damage Modifier`)) _player))
      (`KismetSystemLibrary.Delay` 5.0)
      (set `/Game/Blueprints/ThirdPersonBP/Blueprints/ThirdPersonCharacter.Magic Power` (/ _output_get (`self.Damage Modifier`)) (`self.Player`)))))

(fn `UserConstructionScript`)