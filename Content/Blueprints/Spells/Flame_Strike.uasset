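; Flame Strike spell actor that damages Grunt and Big_Grunt enemies overlapping it.
; On BeginPlay it deducts its mana cost from the player character and derives damage from MagicPower times a modifier.
; Capsule and Cylinder begin-overlap events each subtract that damage directly from enemy HP, with no guard against double hits.
; A Grunt lookup through its own AI controller is stored but unused, and the cooldown-reduction logic is unwired.
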(event `self.ReceiveBeginPlay`
  (`|ExecutionSequence`
    (:`then_0`
      (bind _asai_grunt_controller (cast `/Game/Blueprints/Ai/Ai_grunt_Controller` (`AIBlueprintHelperLibrary.GetAIController` null)))
      (bind _asgrunt (cast `/Game/Blueprints/Enemies/Grunt` (`self.GetOwner` _asai_grunt_controller)))
      (set `self.Grunt` _asgrunt))
    (:`then_1`
      (bind _asthird_person_character (cast `/Game/Blueprints/ThirdPersonBP/Blueprints/ThirdPersonCharacter` (`GameplayStatics.GetPlayerCharacter` 0)))
      (set `/Game/Blueprints/ThirdPersonBP/Blueprints/ThirdPersonCharacter.Mana` (- (`/Game/Blueprints/ThirdPersonBP/Blueprints/ThirdPersonCharacter.Mana` _asthird_person_character) (`self.Mana Cost`)) _asthird_person_character)
      (set `self.Damage` (* (`/Game/Blueprints/ThirdPersonBP/Blueprints/ThirdPersonCharacter.Magic Power` _asthird_person_character) (`self.Damage Modifier`))))))

(event `self.Capsule.OnComponentBeginOverlap`
  (params (OverlappedComponent :type "PrimitiveComponent Object Reference") (OtherActor :type "Actor Object Reference") (OtherComp :type "PrimitiveComponent Object Reference") (OtherBodyIndex :type Integer) (bFromSweep :type Boolean) (SweepResult :type "HitResult Structure (by ref)"))
  (`|ExecutionSequence`
    (:`then_0`
      (bind _asgrunt (cast `/Game/Blueprints/Enemies/Grunt` OtherActor))
      (set `/Game/Blueprints/Enemies/Grunt.HP` (- (`/Game/Blueprints/Enemies/Grunt.HP` _asgrunt) (`self.Damage`)) _asgrunt))
    (:`then_1`
      (bind _asbig_grunt (cast `/Game/Blueprints/Enemies/Big_Grunt` OtherActor))
      (set `/Game/Blueprints/Enemies/Big_Grunt.HP` (- (`/Game/Blueprints/Enemies/Big_Grunt.HP` _asbig_grunt) (`self.Damage`)) _asbig_grunt))))

(event `self.Cylinder.OnComponentBeginOverlap`
  (params (OverlappedComponent :type "PrimitiveComponent Object Reference") (OtherActor :type "Actor Object Reference") (OtherComp :type "PrimitiveComponent Object Reference") (OtherBodyIndex :type Integer) (bFromSweep :type Boolean) (SweepResult :type "HitResult Structure (by ref)"))
  (`|ExecutionSequence`
    (:`then_0`
      (bind _asgrunt (cast `/Game/Blueprints/Enemies/Grunt` OtherActor))
      (set `/Game/Blueprints/Enemies/Grunt.HP` (- (`/Game/Blueprints/Enemies/Grunt.HP` _asgrunt) (`self.Damage`)) _asgrunt))
    (:`then_1`
      (bind _asbig_grunt (cast `/Game/Blueprints/Enemies/Big_Grunt` OtherActor))
      (set `/Game/Blueprints/Enemies/Big_Grunt.HP` (- (`/Game/Blueprints/Enemies/Big_Grunt.HP` _asbig_grunt) (`self.Damage`)) _asbig_grunt))))

(fn `UserConstructionScript`)