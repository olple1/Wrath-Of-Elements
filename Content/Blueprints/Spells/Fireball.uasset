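; Fireball spell actor that costs the player Mana and damages Grunt and Big_Grunt enemies on sphere overlap, then destroys itself.
; BeginPlay reads cost, damage modifier and cooldown from the spells data table, then scales damage by MagicPower and shortens cooldown by CooldownReduction.
; A timed burn on Tick targets only Big_Grunt and is marked as not working; BurnDamage also reads Player before it is assigned.
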(event `self.ReceiveBeginPlay`
  (bind _cooldown_time (`self.Cooldown Time`))
  (`|ExecutionSequence`
    (:`then_0`
      (bind _asai_grunt_controller (cast `/Game/Blueprints/Ai/Ai_grunt_Controller` (`AIBlueprintHelperLibrary.GetAIController` null)))
      (bind _asgrunt (cast `/Game/Blueprints/Enemies/Grunt` (`self.GetOwner` _asai_grunt_controller)))
      (set `self.Grunt` _asgrunt))
    (:`then_1`
      (bind _returnvalue (`|GetDataTableRow` "/Game/Blueprints/Spells_-_Spells.Spells_-_Spells" "Fireball_C")
        (:`then`
          (set `self.Mana Cost` (`.ManaCost_7_C903C12F4449ABCC6E8F80B36C51241A` (break `/Game/Blueprints/SpellsData` _returnvalue)))
          (set `self.Damage Modifier` (`.SpellDamage_3_53CF477246276293E4E13B8EC3A5A41E` (break `/Game/Blueprints/SpellsData` _returnvalue)))
          (set `self.Cooldown Time` (`.Cooldown_20_4E963C174A27AC4E215781B8BC1AD210` (break `/Game/Blueprints/SpellsData` _returnvalue))))))
    (:`then_2`
      (set `self.Burn Damage` (* (`/Game/Blueprints/ThirdPersonBP/Blueprints/ThirdPersonCharacter.Magic Power` (`self.Player`)) 0.02)))
    (:`then_3`
      (bind _asthird_person_character (cast `/Game/Blueprints/ThirdPersonBP/Blueprints/ThirdPersonCharacter` (`GameplayStatics.GetPlayerCharacter` 0)))
      (set `self.Player` _asthird_person_character)
      (set `/Game/Blueprints/ThirdPersonBP/Blueprints/ThirdPersonCharacter.Mana` (- (`/Game/Blueprints/ThirdPersonBP/Blueprints/ThirdPersonCharacter.Mana` _asthird_person_character) (`self.Mana Cost`)) _asthird_person_character)
      (set `self.Damage` (* (`/Game/Blueprints/ThirdPersonBP/Blueprints/ThirdPersonCharacter.Magic Power` _asthird_person_character) (`self.Damage Modifier`)))
      (set `self.Cooldown Time` (- _cooldown_time (* _cooldown_time (/ (`/Game/Blueprints/ThirdPersonBP/Blueprints/ThirdPersonCharacter.Cooldown Reduction` _asthird_person_character) 100.0)))))))

(event `self.Sphere1.OnComponentBeginOverlap`
  (params (OverlappedComponent :type "PrimitiveComponent Object Reference") (OtherActor :type "Actor Object Reference") (OtherComp :type "PrimitiveComponent Object Reference") (OtherBodyIndex :type Integer) (bFromSweep :type Boolean) (SweepResult :type "HitResult Structure (by ref)"))
  (if (`self.ActorHasTag` OtherActor "Grunt")
    (`|ExecutionSequence`
      (:`then_0`
        (bind _asgrunt (cast `/Game/Blueprints/Enemies/Grunt` OtherActor))
        (set `/Game/Blueprints/Enemies/Grunt.HP` (- (`/Game/Blueprints/Enemies/Grunt.HP` _asgrunt) (`self.Damage`)) _asgrunt)
        (`self.K2_DestroyActor` :!label _label))
      (:`then_1`
        (bind _asbig_grunt (cast `/Game/Blueprints/Enemies/Big_Grunt` OtherActor))
        (set `/Game/Blueprints/Enemies/Big_Grunt.HP` (- (`/Game/Blueprints/Enemies/Big_Grunt.HP` _asbig_grunt) (`self.Damage`)) _asbig_grunt)
        (goto _label))
      (:`then_2`
        (set `self.Burning` true)
        (`KismetSystemLibrary.Delay` 5.0)
        (set `self.Burning` false)))))

(event `self.ReceiveTick`
  (params (DeltaSeconds :type "Float (single-precision)"))
  ;[1 1 1] Needs fixing, not working
  (`KismetSystemLibrary.Delay` 1.0)
  (if (`self.Burning`)
    (set `/Game/Blueprints/Enemies/Big_Grunt.HP` (- (`/Game/Blueprints/Enemies/Big_Grunt.HP` (stale `self.Sphere1.OnComponentBeginOverlap` _asbig_grunt)) (`self.Burn Damage`)) (stale `self.Sphere1.OnComponentBeginOverlap` _asbig_grunt))))

(fn `UserConstructionScript`)