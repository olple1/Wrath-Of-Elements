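; RockBlast is a spell Blueprint that instantly kills grunts it touches by setting their HP to zero.
; A Sphere1 overlap checks for the Grunt tag, then casts the overlapping actor to Grunt before changing its HP.
; BeginPlay also tries to cache a Grunt from its own AI controller's owner, but the overlap logic never uses that reference.
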(event `self.ReceiveBeginPlay`
  (`|ExecutionSequence`
    (:`then_0`
      (bind _asai_grunt_controller (cast `/Game/Blueprints/Ai/Ai_grunt_Controller` (`AIBlueprintHelperLibrary.GetAIController` null)))
      (bind _asgrunt (cast `/Game/Blueprints/Enemies/Grunt` (`self.GetOwner` _asai_grunt_controller)))
      (set `self.Grunt` _asgrunt))))

(event `self.Sphere1.OnComponentBeginOverlap`
  (params (OverlappedComponent :type "PrimitiveComponent Object Reference") (OtherActor :type "Actor Object Reference") (OtherComp :type "PrimitiveComponent Object Reference") (OtherBodyIndex :type Integer) (bFromSweep :type Boolean) (SweepResult :type "HitResult Structure (by ref)"))
  (if (`self.ActorHasTag` OtherActor "Grunt")
    (bind _asgrunt (cast `/Game/Blueprints/Enemies/Grunt` OtherActor))
    (set `/Game/Blueprints/Enemies/Grunt.HP` 0.0 _asgrunt)))

(fn `UserConstructionScript`)