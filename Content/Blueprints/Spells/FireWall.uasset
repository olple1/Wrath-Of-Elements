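; Fire Wall spell actor that damages Grunt and Big Grunt enemies entering its box.
; On BeginPlay it reads mana cost, damage modifier and cooldown from the Spells data table, deducts player mana and scales damage by MagicPower.
; Box overlaps add each enemy to a per-type array, then subtract damage directly from HP and remove it.
; Cooldown is loaded, but its reduction logic is unconnected.
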(event `self.ReceiveBeginPlay`
  (`|ExecutionSequence`
    (:`then_1`
      (bind _returnvalue (`|GetDataTableRow` "/Game/Blueprints/Spells_-_Spells.Spells_-_Spells" "FireWall_C")
        (:`then`
          (set `self.Mana Cost` (`.ManaCost_7_C903C12F4449ABCC6E8F80B36C51241A` (break `/Game/Blueprints/SpellsData` _returnvalue)))
          (set `self.Damage Modifier` (`.SpellDamage_3_53CF477246276293E4E13B8EC3A5A41E` (break `/Game/Blueprints/SpellsData` _returnvalue)))
          (set `self.Cooldown Time` (`.Cooldown_20_4E963C174A27AC4E215781B8BC1AD210` (break `/Game/Blueprints/SpellsData` _returnvalue))))))
    (:`then_2`
      (bind _asthird_person_character (cast `/Game/Blueprints/ThirdPersonBP/Blueprints/ThirdPersonCharacter` (`GameplayStatics.GetPlayerCharacter` 0)))
      (set `/Game/Blueprints/ThirdPersonBP/Blueprints/ThirdPersonCharacter.Mana` (- (`/Game/Blueprints/ThirdPersonBP/Blueprints/ThirdPersonCharacter.Mana` _asthird_person_character) (`self.Mana Cost`)) _asthird_person_character)
      (set `self.Damage` (* (`/Game/Blueprints/ThirdPersonBP/Blueprints/ThirdPersonCharacter.Magic Power` _asthird_person_character) (`self.Damage Modifier`))))))

(event `self.Box.OnComponentBeginOverlap`
  (params (OverlappedComponent :type "PrimitiveComponent Object Reference") (OtherActor :type "Actor Object Reference") (OtherComp :type "PrimitiveComponent Object Reference") (OtherBodyIndex :type Integer) (bFromSweep :type Boolean) (SweepResult :type "HitResult Structure (by ref)"))
  (bind _grunt (`self.Grunt`))
  (bind _big_grunt (`self.Big Grunt`))
  (`|ExecutionSequence`
    (:`then_0`
      (bind _asgrunt (cast `/Game/Blueprints/Enemies/Grunt` OtherActor))
      (`KismetArrayLibrary.Array_Add` _grunt _asgrunt)
      (for _array_element _grunt
        (set `/Game/Blueprints/Enemies/Grunt.HP` (- (`/Game/Blueprints/Enemies/Grunt.HP` _array_element) (`self.Damage`)) _array_element)
        (`KismetArrayLibrary.Array_RemoveItem` (`self.Grunt`) _array_element)))
    (:`then_1`
      (bind _asbig_grunt (cast `/Game/Blueprints/Enemies/Big_Grunt` OtherActor))
      (`KismetArrayLibrary.Array_Add` _big_grunt _asbig_grunt)
      (for _array_element_2 _big_grunt
        (set `/Game/Blueprints/Enemies/Big_Grunt.HP` (- (`/Game/Blueprints/Enemies/Big_Grunt.HP` _array_element_2) (`self.Damage`)) _array_element_2)
        (`KismetArrayLibrary.Array_RemoveItem` (`self.Big Grunt`) _array_element_2)))))

(fn `UserConstructionScript`)