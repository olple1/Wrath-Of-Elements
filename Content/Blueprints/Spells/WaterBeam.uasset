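; Water beam spell actor that lives four seconds and damages Grunt and Big_Grunt enemies caught in its capsule.
; On spawn it loads stats from the spell data table, deducts player mana, scales damage and cooldown, and heals the player from remaining mana.
; Tick lengthens the capsule, reattaches to the player's billboard, and uses a Delay to damage overlap-tracked enemies about once per second.
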(event `self.ReceiveBeginPlay`
  (bind _cooldown_time (`self.Cooldown Time`))
  (`|ExecutionSequence`
    (:`then_0`
      (bind _returnvalue (`|GetDataTableRow` "/Game/Blueprints/Spells_-_Spells.Spells_-_Spells" "WaterBeam_C")
        (:`then`
          (set `self.Mana Cost` (`.ManaCost_7_C903C12F4449ABCC6E8F80B36C51241A` (break `/Game/Blueprints/SpellsData` _returnvalue)))
          (set `self.Damage Modifier` (`.SpellDamage_3_53CF477246276293E4E13B8EC3A5A41E` (break `/Game/Blueprints/SpellsData` _returnvalue)))
          (set `self.Cooldown Time` (`.Cooldown_20_4E963C174A27AC4E215781B8BC1AD210` (break `/Game/Blueprints/SpellsData` _returnvalue))))))
    (:`then_1`
      (bind _asthird_person_character (cast `/Game/Blueprints/ThirdPersonBP/Blueprints/ThirdPersonCharacter` (`GameplayStatics.GetPlayerCharacter` 0)))
      (set `self.Player` _asthird_person_character)
      (bind _mana (`/Game/Blueprints/ThirdPersonBP/Blueprints/ThirdPersonCharacter.Mana` _asthird_person_character))
      (set `/Game/Blueprints/ThirdPersonBP/Blueprints/ThirdPersonCharacter.Mana` (- _mana (`self.Mana Cost`)) _asthird_person_character)
      (set `self.Damage` (* (`/Game/Blueprints/ThirdPersonBP/Blueprints/ThirdPersonCharacter.Magic Power` _asthird_person_character) (`self.Damage Modifier`)))
      (set `self.Cooldown Time` (- _cooldown_time (* _cooldown_time (/ (`/Game/Blueprints/ThirdPersonBP/Blueprints/ThirdPersonCharacter.Cooldown Reduction` _asthird_person_character) 100.0))))
      (set `/Game/Blueprints/ThirdPersonBP/Blueprints/ThirdPersonCharacter.HP` (+ (/ _mana 5.0) (`/Game/Blueprints/ThirdPersonBP/Blueprints/ThirdPersonCharacter.HP` (`self.Player`))) _asthird_person_character))
    (:`then_2`
      (`self.SetLifeSpan` 4.0))))

(event `self.Capsule.OnComponentBeginOverlap`
  (params (OverlappedComponent :type "PrimitiveComponent Object Reference") (OtherActor :type "Actor Object Reference") (OtherComp :type "PrimitiveComponent Object Reference") (OtherBodyIndex :type Integer) (bFromSweep :type Boolean) (SweepResult :type "HitResult Structure (by ref)"))
  (if (`self.ActorHasTag` OtherActor "Grunt")
    (`|ExecutionSequence`
      (:`then_0`
        (bind _asgrunt (cast `/Game/Blueprints/Enemies/Grunt` OtherActor))
        (`KismetArrayLibrary.Array_Add` (`self.Grunt`) _asgrunt)
        (set `self.Damage Grunt` true))
      (:`then_1`
        (bind _asbig_grunt (cast `/Game/Blueprints/Enemies/Big_Grunt` OtherActor))
        (`KismetArrayLibrary.Array_Add` (`self.Big Grunt`) _asbig_grunt)
        (set `self.Damage Big Grunt` true)))))

(event `self.Capsule.OnComponentEndOverlap`
  (params (OverlappedComponent :type "PrimitiveComponent Object Reference") (OtherActor :type "Actor Object Reference") (OtherComp :type "PrimitiveComponent Object Reference") (OtherBodyIndex :type Integer))
  (`|ExecutionSequence`
    (:`then_0`
      (bind _asgrunt (cast `/Game/Blueprints/Enemies/Grunt` OtherActor))
      (`KismetArrayLibrary.Array_RemoveItem` (`self.Grunt`) _asgrunt))
    (:`then_1`
      (bind _asbig_grunt (cast `/Game/Blueprints/Enemies/Big_Grunt` OtherActor))
      (`KismetArrayLibrary.Array_RemoveItem` (`self.Big Grunt`) _asbig_grunt))))

(event `self.ReceiveTick`
  (params (DeltaSeconds :type "Float (single-precision)"))
  (bind _capsule (`self.Capsule`))
  (`|ExecutionSequence`
    (:`then_0`
      (`CapsuleComponent.SetCapsuleHalfHeight` _capsule (+ (`CapsuleComponent.CapsuleHalfHeight` _capsule) 100.0) true))
    (:`then_1`
      (`KismetSystemLibrary.Delay` 1.0)
      (`|ExecutionSequence`
        (:`then_0`
          (if (`self.Damage Grunt`)
            (for _array_element (`self.Grunt`)
              (set `/Game/Blueprints/Enemies/Grunt.HP` (- (`/Game/Blueprints/Enemies/Grunt.HP` _array_element) (`self.Damage`)) _array_element))))
        (:`then_1`
          (if (`self.Damage Big Grunt`)
            (for _array_element_2 (`self.Big Grunt`)
              (set `/Game/Blueprints/Enemies/Big_Grunt.HP` (- (`/Game/Blueprints/Enemies/Big_Grunt.HP` _array_element_2) (`self.Damage`)) _array_element_2))))))
    (:`then_2`
      (`self.K2_AttachToComponent` (`/Game/Blueprints/ThirdPersonBP/Blueprints/ThirdPersonCharacter.Billboard` (`self.Player`)) "None" "KeepWorld" "KeepWorld" "KeepRelative"))))

(fn `UserConstructionScript`)