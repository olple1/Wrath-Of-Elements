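; Kill volume actor that kills enemies that leave the play area.
; Its Box overlap event tries casting the other actor to Grunt, Big_Grunt and Ranged_Grunt in sequence.
; A matching enemy is appended to that type's array, then every member of the array has its HP set to zero.
; The arrays are never cleared here, so earlier entries are zeroed again on each new matching overlap.
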(event `self.Box.OnComponentBeginOverlap`
  (params (OverlappedComponent :type "PrimitiveComponent Object Reference") (OtherActor :type "Actor Object Reference") (OtherComp :type "PrimitiveComponent Object Reference") (OtherBodyIndex :type Integer) (bFromSweep :type Boolean) (SweepResult :type "HitResult Structure (by ref)"))
  (bind _ranged_grunt (`self.Ranged Grunt`))
  (`|ExecutionSequence`
    (:`then_0`
      (bind _asgrunt (cast `/Game/Blueprints/Enemies/Grunt` OtherActor))
      (`KismetArrayLibrary.Array_Add` (`self.Grunt`) _asgrunt)
      (for _array_element (`self.Grunt`)
        (set `/Game/Blueprints/Enemies/Grunt.HP` 0.0 _array_element)))
    (:`then_1`
      (bind _asbig_grunt (cast `/Game/Blueprints/Enemies/Big_Grunt` OtherActor))
      (`KismetArrayLibrary.Array_Add` (`self.Big Grunt`) _asbig_grunt)
      (for _array_element_2 (`self.Big Grunt`)
        (set `/Game/Blueprints/Enemies/Big_Grunt.HP` 0.0 _array_element_2)))
    (:`then_2`
      (bind _asranged_grunt (cast `/Game/Blueprints/Enemies/Ranged_Grunt` OtherActor))
      (`KismetArrayLibrary.Array_Add` _ranged_grunt _asranged_grunt)
      (for _array_element_3 _ranged_grunt
        (set `/Game/Blueprints/Enemies/Ranged_Grunt.HP` 0.0 _array_element_3)))))

(fn `UserConstructionScript`)