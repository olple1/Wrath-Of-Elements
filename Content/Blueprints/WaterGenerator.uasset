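; Construction-script generator that builds a body of water along an editable spline from spline mesh components.
; It resizes WaterDataArray to the spline point count, then BuildWater adds a WaterMesh piece per loop index, bent between that point and the next.
; Each piece takes start roll and width from its point's data, but end roll and width always come from the first entry.
; Event graph is unused.
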(fn `Array`
  (bind _waterdataarray (`self.WaterDataArray`))
  (`/Engine/EditorBlueprintResources/StandardMacros.CompareInt` (`KismetArrayLibrary.Array_Length` (`self.WaterDataArray`)) (`self.Number Of Spline Points`) :!label _label
    (:`>`
      (`KismetArrayLibrary.Array_Remove` _waterdataarray (`KismetArrayLibrary.Array_LastIndex` _waterdataarray))
      (goto _label))
    (:`<`
      (`KismetArrayLibrary.Array_Add` (`self.WaterDataArray`))
      (goto _label))))

(fn `Build Water`
  (params (LoopIndex :type Integer) (`Water Mesh` :type "StaticMesh Object Reference"))
  (locals (`Local CurrentLoopIndex` :type Integer) (`Local NextLoopIndex` :type Integer) (`Local Water Mesh` :type "StaticMesh Object Reference") (`Local Start Location` :type "Vector Structure") (`Local Start Tangent` :type "Vector Structure") (`Local End Location` :type "Vector Structure") (`Local End Tangent` :type "Vector Structure") (`Local CurrentSplineMesh` :type "SplineMeshComponent Object Reference") (`Local Start Roll` :type "Float (double-precision)") (`Local Start Scale` :type "Vector2D Structure") (`Local End Roll` :type "Float (double-precision)") (`Local End Scale` :type "Vector2D Structure"))
  (bind (_location _tangent) (`SplineComponent.GetLocationAndTangentAtSplinePoint` (`self.Spline`) (`local.Local NextLoopIndex`) "Local"))
  (bind (_location_2 _tangent_2) (`SplineComponent.GetLocationAndTangentAtSplinePoint` (`self.Spline`) (`local.Local CurrentLoopIndex`) "Local"))
  (bind (_output_waterturn _output_waterwidth) (break `/Game/Blueprints/Water_Data` (`|GetArrayItem` (`self.WaterDataArray`))))
  (bind (_output_waterturn_2 _output_waterwidth_2) (break `/Game/Blueprints/Water_Data` (`|GetArrayItem` (`self.WaterDataArray`) (`local.Local CurrentLoopIndex`))))
  (set `local.Local CurrentLoopIndex` LoopIndex)
  (set `local.Local NextLoopIndex` (+ LoopIndex 1))
  (set `local.Local Water Mesh` `Water Mesh`)
  (`|ExecutionSequence`
    (:`then_0`
      (set `local.Local Start Location` _location_2)
      (set `local.Local Start Tangent` _tangent_2)
      (set `local.Local End Location` _location)
      (set `local.Local End Tangent` _tangent)
      (set `local.Local Start Roll` _output_waterturn_2)
      (set `local.Local Start Scale` (`KismetMathLibrary.MakeVector2D` _output_waterwidth_2))
      (set `local.Local End Roll` _output_waterturn)
      (set `local.Local End Scale` (`KismetMathLibrary.MakeVector2D` _output_waterwidth)))
    (:`then_1`
      (bind _returnvalue (`AddComponent|NODE_AddSplineMeshComponent-0`))
      (set `local.Local CurrentSplineMesh` _returnvalue)
      (`StaticMeshComponent.SetStaticMesh` (`local.Local CurrentSplineMesh`) (`local.Local Water Mesh`))
      (`SplineMeshComponent.SetStartAndEnd` (`local.Local CurrentSplineMesh`) (`local.Local Start Location`) (`local.Local Start Tangent`) (`local.Local End Location`) (`local.Local End Tangent`) true)
      (`SplineMeshComponent.SetStartRoll` (`local.Local CurrentSplineMesh`) (`local.Local Start Roll`) true)
      (`SplineMeshComponent.SetEndRoll` (`local.Local CurrentSplineMesh`) (`local.Local End Roll`) true)
      (`SplineMeshComponent.SetStartScale` (`local.Local CurrentSplineMesh`) (`local.Local Start Scale`) true)
      (`SplineMeshComponent.SetEndScale` (`local.Local CurrentSplineMesh`) (`local.Local End Scale`) true))))

(fn `Spline Number`
  (set `self.Number Of Spline Points` (`SplineComponent.GetNumberOfSplinePoints` (`self.Spline`))))

(fn `UserConstructionScript`
  (`|ExecutionSequence`
    (:`then_0`
      (`self.Spline Number`))
    (:`then_1`
      (`self.Array`))
    (:`then_2`
      (for _index (range (+ (`self.Number Of Spline Points`) 1))
        (`self.Build Water` _index (`self.Water Mesh`))))))