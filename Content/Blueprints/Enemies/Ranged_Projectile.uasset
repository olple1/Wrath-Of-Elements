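; Enemy ranged projectile that damages the ThirdPersonCharacter when its capsule overlaps them.
; A DoOnce limits it to one hit, which subtracts Damage minus the character's Armor from HP and updates the HUD.
; At zero HP or below it calls CallGameWin on the WrathOfElements game mode without destroying itself.
; Otherwise, including when Armor exceeds Damage, the projectile destroys itself.
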(event `self.Capsule.OnComponentBeginOverlap`
  (params (OverlappedComponent :type "PrimitiveComponent Object Reference") (OtherActor :type "Actor Object Reference") (OtherComp :type "PrimitiveComponent Object Reference") (OtherBodyIndex :type Integer) (bFromSweep :type Boolean) (SweepResult :type "HitResult Structure (by ref)"))
  (bind _asthird_person_character (cast `/Game/Blueprints/ThirdPersonBP/Blueprints/ThirdPersonCharacter` OtherActor))
  (`/Engine/EditorBlueprintResources/StandardMacros.DoOnce` false
    (:`Completed`
      (bind _returnvalue (- (`self.Damage`) (`/Game/Blueprints/ThirdPersonBP/Blueprints/ThirdPersonCharacter.Armor` _asthird_person_character)))
      (if (> 0.0 _returnvalue)
        (`self.K2_DestroyActor`)
        (else
          (bind _output_get (set `/Game/Blueprints/ThirdPersonBP/Blueprints/ThirdPersonCharacter.HP` (- (`/Game/Blueprints/ThirdPersonBP/Blueprints/ThirdPersonCharacter.HP` _asthird_person_character) _returnvalue) _asthird_person_character))
          (bind _hud (`/Game/Blueprints/ThirdPersonBP/Blueprints/ThirdPersonCharacter.HUD` _asthird_person_character))
          (`/Game/Blueprints/UI/HUD.Changing HP` _hud)
          (`/Game/Blueprints/UI/HUD.Damage Player` _hud)
          (if (<= _output_get 0.0)
            (bind _aswrath_of_elements_game_mode (cast `/Game/Blueprints/WrathOfElements_GameMode` (`GameplayStatics.GetGameMode`)))
            (`/Game/Blueprints/WrathOfElements_GameMode.Game Win` _aswrath_of_elements_game_mode)
            (else
              (`self.K2_DestroyActor`))))))))

(fn `UserConstructionScript`)