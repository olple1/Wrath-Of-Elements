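; Enemy spawner actor that creates a limited number of grunt AI pawns at its own location.
; Tick feeds a Delay of SpawnSpeed, which acts as a repeating timer and spawns only while SpawnedAmount is below SpawnCount.
; Each spawn randomly picks Big_Grunt or Grunt, starts it on the shared Grunt behavior tree and increments the counter.
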(event `self.ReceiveTick`
  (params (DeltaSeconds :type "Float (single-precision)"))
  (`KismetSystemLibrary.Delay` (`self.Spawn Speed`))
  (`/Engine/EditorBlueprintResources/StandardMacros.CompareInt` (`self.Spawn Count`) (`self.Spawned amount`)
    (:`>`
      (switch `int` (`KismetMathLibrary.RandomIntegerInRange` 0 1)
        (:`0`
          (set `self.enemy` "/Game/Blueprints/Enemies/Big_Grunt.Big_Grunt_C"))
        (:`1`
          (set `self.enemy` "/Game/Blueprints/Enemies/Grunt.Grunt_C")))
      (`AIBlueprintHelperLibrary.SpawnAIFromClass` (`self.enemy`) "/Game/Blueprints/Ai/Grunt.Grunt" (`self.K2_GetActorLocation`))
      (set `self.Spawned amount` (+ (`self.Spawned amount`) 1)))))

(fn `UserConstructionScript`)