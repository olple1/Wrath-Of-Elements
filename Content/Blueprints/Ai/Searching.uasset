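; Behavior tree task for a Grunt AI that searches around the pawn's last seen location.
; The Searching event waits, moves to a random reachable nav point near LastSeen, and repeats through a DoN gate whose counter check can set the AiState blackboard enum and finish the task.
; As wired, execution only caches the Grunt: the move to LastSeen that would start Searching is disconnected.
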(event `self.ReceiveExecuteAI`
  (params (OwnerController :type "AIController Object Reference") (ControlledPawn :type "Pawn Object Reference"))
  (bind _asgrunt (cast `/Game/Blueprints/Enemies/Grunt` ControlledPawn)))

(event `Searching`
  (`KismetSystemLibrary.Delay` 3.0)
  (bind _outactors (`GameplayStatics.GetAllActorsOfClass` "/Script/NavigationSystem.RecastNavMesh"))
  (`|AIMoveTo` null (`NavigationSystemV1.K2_GetRandomReachablePointInRadius` (`/Game/Blueprints/Enemies/Grunt.Last Seen` (stale `self.ReceiveExecuteAI` _asgrunt)) 1200.0 (`|GetArrayItem` _outactors) null) null
    (:`OnSuccess`
      (bind _counter (`/Engine/EditorBlueprintResources/StandardMacros.Do N` 3 :!label _label)
        (:`Exit`
          (if (<= _counter 0)
            (`BTFunctionLibrary.SetBlackboardValueAsEnum` (`self.Ai State`) (enumliteral `/Game/Blueprints/Ai/AI_State` "NewEnumerator5"))
            (`self.Reset1`)
            (`self.FinishExecute` true)
            (else
              (`self.Searching`))))))))

(event `Reset1`
  (goto _label :!via `Reset`))