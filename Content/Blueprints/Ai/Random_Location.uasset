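; Behavior tree task that picks a random wander point for grunt enemies and stores it in the RandomLocation blackboard key.
; A Sequence tries casts to Big_Grunt, Grunt and Ranged_Grunt, each branch repeating the same logic.
; The matching branch queries the first RecastNavMesh for a navigable point within a fixed radius of the pawn, then finishes successfully.
; No failure finish exists for other pawn types.
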(event `self.ReceiveExecuteAI`
  (params (OwnerController :type "AIController Object Reference") (ControlledPawn :type "Pawn Object Reference"))
  (`|ExecutionSequence`
    (:`then_0`
      (bind _asbig_grunt (cast `/Game/Blueprints/Enemies/Big_Grunt` ControlledPawn))
      (bind _outactors (`GameplayStatics.GetAllActorsOfClass` "/Script/NavigationSystem.RecastNavMesh"))
      (bind _randomlocation (`NavigationSystemV1.K2_GetRandomLocationInNavigableRadius` (`Actor.K2_GetActorLocation` _asbig_grunt) 2000.0 (`|GetArrayItem` _outactors) "/Script/AIModule.NavFilter_AIControllerDefault"))
      (`BTFunctionLibrary.SetBlackboardValueAsVector` (`self.Random Location`) _randomlocation))
    (:`then_1`
      (bind _asgrunt (cast `/Game/Blueprints/Enemies/Grunt` ControlledPawn))
      (bind _outactors_2 (`GameplayStatics.GetAllActorsOfClass` "/Script/NavigationSystem.RecastNavMesh"))
      (bind _randomlocation_2 (`NavigationSystemV1.K2_GetRandomLocationInNavigableRadius` (`Actor.K2_GetActorLocation` _asgrunt) 2000.0 (`|GetArrayItem` _outactors_2) "/Script/AIModule.NavFilter_AIControllerDefault"))
      (`BTFunctionLibrary.SetBlackboardValueAsVector` (`self.Random Location`) _randomlocation_2))
    (:`then_2`
      (bind _asranged_grunt (cast `/Game/Blueprints/Enemies/Ranged_Grunt` ControlledPawn))
      (bind _outactors_3 (`GameplayStatics.GetAllActorsOfClass` "/Script/NavigationSystem.RecastNavMesh"))
      (bind _randomlocation_3 (`NavigationSystemV1.K2_GetRandomLocationInNavigableRadius` (`Actor.K2_GetActorLocation` _asranged_grunt) 2000.0 (`|GetArrayItem` _outactors_3) "/Script/AIModule.NavFilter_AIControllerDefault"))
      (`BTFunctionLibrary.SetBlackboardValueAsVector` (`self.Random Location`) _randomlocation_3)))
  (`self.FinishExecute` true))