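; Energy blast actor fired with the player's ranged stats: on spawn it copies RangedDamage and Scale from ThirdPerson_Character and attaches an Energy_Ball emitter to its sphere.
; Overlapping a Target_Dummy or AiChar swaps the ball for an impact emitter, then destroys the actor after a one-second delay.
; Damage is only stored here, not applied.
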(event `self.ReceiveBeginPlay`
  (bind _sphere (`self.Sphere`))
  (bind _asthird_person_character (cast `/Game/Blueprints/ThirdPerson_Character` (`GameplayStatics.GetPlayerCharacter` 0)))
  (bind _scale (`/Game/Blueprints/ThirdPerson_Character.Scale` _asthird_person_character))
  (bind _returnvalue (`GameplayStatics.SpawnEmitterAttached` "/Game/Particles/Energy_Ball.Energy_Ball" _sphere "None" (`SceneComponent.RelativeLocation` _sphere) (struct) _scale))
  (set `self.Damage` (`/Game/Blueprints/ThirdPerson_Character.Ranged Damage` _asthird_person_character))
  (`SceneComponent.SetRelativeScale3D` (`self.Sphere`) _scale))

(event `self.Sphere.OnComponentBeginOverlap`
  (params (OverlappedComponent :type "PrimitiveComponent Object Reference") (OtherActor :type "Actor Object Reference") (OtherComp :type "PrimitiveComponent Object Reference") (OtherBodyIndex :type Integer) (bFromSweep :type Boolean) (SweepResult :type "HitResult Structure (by ref)"))
  (bind _sphere (`self.Sphere`))
  (`|ExecutionSequence`
    (:`then_0`
      (cast `/Game/Blueprints/Target_Dummy` OtherActor))
    (:`then_1`
      (cast `/Game/Ai/AiChar` OtherActor)))
  (bind _returnvalue (`GameplayStatics.SpawnEmitterAttached` "/Engine/Tutorial/SubEditors/TutorialAssets/TutorialParticleSystem.TutorialParticleSystem" _sphere "None" (`SceneComponent.RelativeLocation` _sphere) (struct) (`/Game/Blueprints/ThirdPerson_Character.Scale` (stale `self.ReceiveBeginPlay` _asthird_person_character)) "KeepRelativeOffset" false))
  (`ActorComponent.K2_DestroyComponent` (stale `self.ReceiveBeginPlay` _returnvalue))
  (`KismetSystemLibrary.Delay` 1.0)
  (if (`KismetSystemLibrary.IsValid` _returnvalue)
    (`ActorComponent.K2_DestroyComponent` _returnvalue)
    (`self.K2_DestroyActor`)
    (else
      (`self.K2_DestroyActor`))))

(fn `UserConstructionScript`)