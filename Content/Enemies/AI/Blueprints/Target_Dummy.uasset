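; A target dummy enemy that takes damage from Energy_Blast projectiles and is destroyed when its health runs out.
; When an actor overlaps its Box, it casts that actor to Energy_Blast and subtracts the blast's Damage from Hp.
; The remaining Hp is shown on a TextRender, and the actor destroys itself at zero or below.
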(event `self.Box.OnComponentBeginOverlap`
  (params (OverlappedComponent :type "PrimitiveComponent Object Reference") (OtherActor :type "Actor Object Reference") (OtherComp :type "PrimitiveComponent Object Reference") (OtherBodyIndex :type Integer) (bFromSweep :type Boolean) (SweepResult :type "HitResult Structure (by ref)"))
  (bind _hp (`self.Hp`))
  (bind _asenergy_blast (cast `/Game/Blueprints/Energy_Blast` OtherActor))
  (bind _output_get (set `self.Hp` (- _hp (`/Game/Blueprints/Energy_Blast.Damage` _asenergy_blast))))
  (`TextRenderComponent.K2_SetText` (`self.TextRender`) (`KismetTextLibrary.Conv_IntToText` _hp))
  (if (<= _output_get 0)
    (`self.K2_DestroyActor`)))

(fn `UserConstructionScript`)