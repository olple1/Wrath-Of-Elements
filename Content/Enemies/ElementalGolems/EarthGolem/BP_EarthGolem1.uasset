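; Earth golem enemy that hurts the player while they overlap its damage box and, on death, grants EXP to the player and the saved selected element.
; Tick drives the HP display, delayed contact damage minus armor, burn ticks and death.
; Capsule overlaps cast to each spell type: fire spells set tiered burns, while other spells change HP only under Passive2.
; Passive flags alter burn stacking, decay, damage and a death explosion.
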(event `self.ReceiveBeginPlay`
  (bind _returnvalue (`KismetTextLibrary.Conv_DoubleToText` (`self.HP`) "HalfToEven"))
  (bind _returnvalue_2 (`GameplayStatics.LoadGameFromSlot` "Spell_Selection"))
  (bind _output_get (set `self.Save Game` _returnvalue_2))
  (bind _asspell_selection (cast `/Game/Blueprints/Spell_Selection` _output_get))
  (set `self.Fire Selected` (`/Game/Blueprints/Spell_Selection.Fire Element Selected` _asspell_selection))
  (set `self.Air Selected` (`/Game/Blueprints/Spell_Selection.Air Element Selected` _asspell_selection))
  (set `self.Water Selected` (`/Game/Blueprints/Spell_Selection.Water Element Selected` _asspell_selection))
  (set `self.Earth Selected` (`/Game/Blueprints/Spell_Selection.Earth Element Selected` _asspell_selection))
  (bind _asthird_person_character (cast `/Game/Blueprints/ThirdPersonBP/Blueprints/ThirdPersonCharacter` (`GameplayStatics.GetPlayerCharacter` 0)))
  (set `self.Character` _asthird_person_character)
  (`TextRenderComponent.K2_SetText` (`self.Golem Max HP`) _returnvalue)
  (`TextRenderComponent.K2_SetText` (`self.Golem current HP`) _returnvalue))

(event `self.ReceiveTick`
  (params (DeltaSeconds :type "Float (single-precision)"))
  (bind _character (`self.Character`))
  (bind _damage (`self.Damage`))
  (bind _burn_count (`self.Burn Count`))
  (bind _exp (`self.EXP`))
  (`|ExecutionSequence`
    (:`then_0`
      (`TextRenderComponent.K2_SetText` (`self.Golem current HP`) (`KismetTextLibrary.Conv_DoubleToText` (`self.HP`) "HalfToEven"))
      (if (<= (`self.HP`) 0.0)
        (`/Engine/EditorBlueprintResources/StandardMacros.DoOnce` false
          (:`Completed`
            (if (`self.Passive 4`)
              (if (>= (`self.Burn Count`) 4.0)
                (`|SpawnActorFromClass` "/Game/Blueprints/Spells/Fire/Passive_Explosion.Passive_Explosion_C" (`KismetMathLibrary.Conv_VectorToTransform` (`self.K2_GetActorLocation`)) "AlwaysSpawn" "OverrideRootScale" null null)))
            ;[1 1 1] EXP
            (set `/Game/Blueprints/ThirdPersonBP/Blueprints/ThirdPersonCharacter.EXP` (+ (`/Game/Blueprints/ThirdPersonBP/Blueprints/ThirdPersonCharacter.EXP` _character) _exp) _character)
            (`|ExecutionSequence`
              (:`then_0`
                (if (`self.Fire Selected`)
                  (set `/Game/Blueprints/ThirdPersonBP/Blueprints/ThirdPersonCharacter.Fire Magic EXP ` (+ (`/Game/Blueprints/ThirdPersonBP/Blueprints/ThirdPersonCharacter.Fire Magic EXP ` _character) _exp) _character)
                  (`self.K2_DestroyActor` :!label _label)))
              (:`then_1`
                (if (`self.Air Selected`)
                  (set `/Game/Blueprints/ThirdPersonBP/Blueprints/ThirdPersonCharacter.Air Magic EXP` (+ (`/Game/Blueprints/ThirdPersonBP/Blueprints/ThirdPersonCharacter.Air Magic EXP` _character) _exp) _character)
                  (goto _label)))
              (:`then_2`
                (if (`self.Water Selected`)
                  (set `/Game/Blueprints/ThirdPersonBP/Blueprints/ThirdPersonCharacter.Water Magic EXP` (+ (`/Game/Blueprints/ThirdPersonBP/Blueprints/ThirdPersonCharacter.Water Magic EXP` _character) _exp) _character)
                  (goto _label)))
              (:`then_3`
                (if (`self.Earth Selected`)
                  (set `/Game/Blueprints/ThirdPersonBP/Blueprints/ThirdPersonCharacter.Earth Magic EXP` (+ (`/Game/Blueprints/ThirdPersonBP/Blueprints/ThirdPersonCharacter.Earth Magic EXP` _character) _exp) _character)
                  (goto _label))))))))
    (:`then_1`
      (if (`self.Dealing dmg`)
        (`KismetSystemLibrary.Delay` 0.5)
        (bind _armor (`/Game/Blueprints/ThirdPersonBP/Blueprints/ThirdPersonCharacter.Armor` (stale `self.Damage Box.OnComponentBeginOverlap` _asthird_person_character)))
        (bind _returnvalue (- _damage _armor))
        (if (not (> 0.0 _returnvalue))
          (if (`self.Passive 2`)
            (set `/Game/Blueprints/ThirdPersonBP/Blueprints/ThirdPersonCharacter.HP` (- (* _damage (+ (* (`self.Burn Count`) 0.1) 1.0)) _armor) (stale `self.Damage Box.OnComponentBeginOverlap` _asthird_person_character))
            (else
              (bind _output_get (set `/Game/Blueprints/ThirdPersonBP/Blueprints/ThirdPersonCharacter.HP` (- (`/Game/Blueprints/ThirdPersonBP/Blueprints/ThirdPersonCharacter.HP` (stale `self.Damage Box.OnComponentBeginOverlap` _asthird_person_character)) _returnvalue) (stale `self.Damage Box.OnComponentBeginOverlap` _asthird_person_character)))))
          (bind _hud (`/Game/Blueprints/ThirdPersonBP/Blueprints/ThirdPersonCharacter.HUD` (stale `self.Damage Box.OnComponentBeginOverlap` _asthird_person_character)))
          (`/Game/Blueprints/UI/HUD.Changing HP` _hud)
          (`/Game/Blueprints/UI/HUD.Damage Player` _hud)
          (if (<= _output_get 0.0)
            (bind _aswrath_of_elements_game_mode (cast `/Game/Blueprints/WrathOfElements_GameMode` (`GameplayStatics.GetGameMode`)))
            (`/Game/Blueprints/WrathOfElements_GameMode.Game Win` _aswrath_of_elements_game_mode)))))
    (:`then_2`
      (`KismetSystemLibrary.Delay` 1.0)
      (if (`self.Burning`)
        (set `self.HP` (- (`self.HP`) (`self.Burn Damage`)))))
    (:`then_3`
      (if (`self.Passive 3`)
        (`KismetSystemLibrary.Delay` 2.0)
        (set `self.Burn Count` (- _burn_count 1.0))
        (if (>= 0.0 _burn_count)
          (set `self.Burning` false))))))

(event `self.Damage Box.OnComponentBeginOverlap`
  (params (OverlappedComponent :type "PrimitiveComponent Object Reference") (OtherActor :type "Actor Object Reference") (OtherComp :type "PrimitiveComponent Object Reference") (OtherBodyIndex :type Integer) (bFromSweep :type Boolean) (SweepResult :type "HitResult Structure (by ref)"))
  (bind _asthird_person_character (cast `/Game/Blueprints/ThirdPersonBP/Blueprints/ThirdPersonCharacter` OtherActor))
  (set `self.Dealing dmg` true))

(event `self.Damage Box.OnComponentEndOverlap`
  (params (OverlappedComponent :type "PrimitiveComponent Object Reference") (OtherActor :type "Actor Object Reference") (OtherComp :type "PrimitiveComponent Object Reference") (OtherBodyIndex :type Integer))
  (cast `/Game/Blueprints/ThirdPersonBP/Blueprints/ThirdPersonCharacter` OtherActor)
  (set `self.Dealing dmg` false))

(event `self.CapsuleComponent.OnComponentBeginOverlap`
  (params (OverlappedComponent :type "PrimitiveComponent Object Reference") (OtherActor :type "Actor Object Reference") (OtherComp :type "PrimitiveComponent Object Reference") (OtherBodyIndex :type Integer) (bFromSweep :type Boolean) (SweepResult :type "HitResult Structure (by ref)"))
  (bind _passive_3 (`self.Passive 3`))
  (bind _passive_3_2 (`self.Passive 3`))
  (bind _passive_3_3 (`self.Passive 3`))
  (bind _hp (`self.HP`))
  (bind _returnvalue (* (`self.Burn Count`) 0.1))
  ;[1 1 1] Burn Damage
  (`|ExecutionSequence`
    (:`then_0`
      (bind _asfireball (cast `/Game/Blueprints/Spells/Fire/Fireball` OtherActor))
      (set `self.Taking Damage` true)
      (`|ExecutionSequence`
        (:`then_0`
          (`/Engine/EditorBlueprintResources/StandardMacros.CompareFloat` (`self.Burn Count`) 1.0
            (:`>`
              (if _passive_3
                (if _passive_3 :!label _label_2
                  (set `self.Burn Count` (+ (`self.Burn Count`) 1.0))
                  (else
                    (set `self.Burn Count` 1.0)))
                (set `self.Burn Damage` (* (* (`/Game/Blueprints/Spells/Fire/Fireball.Damage` _asfireball) 0.02) (`self.Burn Count`)))))
            (:`==`
              (set `self.Strongest burn` 1.0 :!label _label_3)
              (goto _label_2))
            (:`<`
              (goto _label_3)))
          (`self.K2_DestroyActor` _asfireball)
          (set `self.Burning` true)
          (`KismetSystemLibrary.Delay` 3.0)
          (if (not (`self.Passive 3`))
            (if (>= (`self.Burn Count`) (`self.Strongest burn`)) :!label _label_4
              (set `self.Burning` false :!label _label_5)
              (set `self.Burn Count` 0.0)
              (set `self.Strongest burn` 0.0))))
        (:`then_1`
          (if (`self.Passive 2`)
            (set `self.HP` (- (* (`/Game/Blueprints/Spells/Fire/Fireball.Damage` _asfireball) _returnvalue) _hp))))
        (:`then_2`
          (`KismetSystemLibrary.Delay` 0.5)
          (set `self.Taking Damage` false))))
    (:`then_1`
      (bind _asfire_wall (cast `/Game/Blueprints/Spells/Fire/FireWall` OtherActor))
      (set `self.Taking Damage` true)
      (`|ExecutionSequence`
        (:`then_0`
          (`/Engine/EditorBlueprintResources/StandardMacros.CompareFloat` (`self.Burn Count`) 2.0
            (:`>`
              (if _passive_3_2
                (if _passive_3_2 :!label _label_6
                  (set `self.Burn Count` (+ (`self.Burn Count`) 2.0))
                  (else
                    (set `self.Burn Count` 2.0)))
                (set `self.Burn Damage` (* (* (`/Game/Blueprints/Spells/Fire/FireWall.Damage` _asfire_wall) 0.02) (`self.Burn Count`)))
                (set `self.Burning` true)
                (`KismetSystemLibrary.Delay` 5.0)
                (if (not (`self.Passive 3`))
                  (goto _label_4))))
            (:`==`
              (set `self.Strongest burn` 2.0 :!label _label_7)
              (goto _label_6))
            (:`<`
              (goto _label_7))))
        (:`then_1`
          (if (`self.Passive 2`)
            (set `self.HP` (- (* (`/Game/Blueprints/Spells/Fire/FireWall.Damage` _asfire_wall) _returnvalue) _hp))))
        (:`then_2`
          (`KismetSystemLibrary.Delay` 0.5)
          (set `self.Taking Damage` false))))
    (:`then_2`
      (bind _asflame_strike (cast `/Game/Blueprints/Spells/Fire/Flame_Strike` OtherActor))
      (set `self.Taking Damage` true)
      (`|ExecutionSequence`
        (:`then_0`
          (`/Engine/EditorBlueprintResources/StandardMacros.CompareFloat` (`self.Burn Count`) 3.0
            (:`>`
              (if _passive_3_3
                (if _passive_3_3 :!label _label_8
                  (set `self.Burn Count` (+ (`self.Burn Count`) 3.0))
                  (else
                    (set `self.Burn Count` 3.0)))
                (set `self.Burn Damage` (* (* (`/Game/Blueprints/Spells/Fire/Flame_Strike.Damage` _asflame_strike) 0.02) (`self.Burn Count`)))
                (set `self.Burning` true)
                (`KismetSystemLibrary.Delay` 7.0)
                (if (not (`self.Passive 3`))
                  (goto _label_4))))
            (:`==`
              (set `self.Strongest burn` 3.0 :!label _label_9)
              (goto _label_8))
            (:`<`
              (goto _label_9))))
        (:`then_1`
          (if (`self.Passive 2`)
            (set `self.HP` (- (* (`/Game/Blueprints/Spells/Fire/Flame_Strike.Damage` _asflame_strike) _returnvalue) _hp))))
        (:`then_2`
          (`KismetSystemLibrary.Delay` 0.5)
          (set `self.Taking Damage` false))))
    (:`then_3`
      (bind _asmeteor (cast `/Game/Blueprints/Spells/Fire/Meteor` OtherActor))
      (set `self.Taking Damage` true)
      (`|ExecutionSequence`
        (:`then_0`
          (set `self.Strongest burn` 4.0)
          (if (`self.Passive 3`)
            (set `self.Burn Count` (+ (`self.Burn Count`) 4.0))
            (else
              (set `self.Burn Count` 4.0)))
          (set `self.Burn Damage` (* (* (`/Game/Blueprints/Spells/Fire/Meteor.Damage` _asmeteor) 0.02) (`self.Burn Count`)))
          (set `self.Burning` true)
          (`KismetSystemLibrary.Delay` 10.0)
          (if (not (`self.Passive 3`))
            (goto _label_5)))
        (:`then_1`
          (if (`self.Passive 2`)
            (set `self.HP` (- (* (`/Game/Blueprints/Spells/Fire/Meteor.Damage` _asmeteor) _returnvalue) _hp))))
        (:`then_2`
          (`KismetSystemLibrary.Delay` 0.5)
          (set `self.Taking Damage` false))))
    (:`then_4`
      (bind _asearthquake (cast `/Game/Blueprints/Spells/Earth/Earthquake` OtherActor))
      (set `self.Taking Damage` true)
      (`|ExecutionSequence`
        (:`then_0`
          (if (`self.Passive 2`)
            (set `self.HP` (- (* (`/Game/Blueprints/Spells/Earth/Earthquake.Damage` _asearthquake) _returnvalue) _hp))))
        (:`then_1`
          (`KismetSystemLibrary.Delay` 0.5)
          (set `self.Taking Damage` false))))
    (:`then_5`
      (bind _asrock_blast (cast `/Game/Blueprints/Spells/Earth/RockBlast` OtherActor))
      (set `self.Taking Damage` true)
      (`|ExecutionSequence`
        (:`then_0`
          (if (`self.Passive 2`)
            (set `self.HP` (- (* (`/Game/Blueprints/Spells/Earth/RockBlast.Damage` _asrock_blast) _returnvalue) _hp))))
        (:`then_1`
          (`KismetSystemLibrary.Delay` 0.5)
          (set `self.Taking Damage` false))))
    (:`then_6`
      (bind _asaftershock (cast `/Game/Blueprints/Spells/Earth/Aftershock` OtherActor))
      (set `self.Taking Damage` true)
      (`|ExecutionSequence`
        (:`then_0`
          (if (`self.Passive 2`)
            (set `self.HP` (- (* (`/Game/Blueprints/Spells/Earth/Aftershock.Damage` _asaftershock) _returnvalue) _hp))))
        (:`then_1`
          (`KismetSystemLibrary.Delay` 0.5)
          (set `self.Taking Damage` false))))
    (:`then_7`
      (bind _aswater_bolt (cast `/Game/Blueprints/Spells/Water/WaterBolt` OtherActor))
      (set `self.Taking Damage` true)
      (`|ExecutionSequence`
        (:`then_0`
          (if (`self.Passive 2`)
            (set `self.HP` (- (* (`/Game/Blueprints/Spells/Water/WaterBolt.Damage` _aswater_bolt) _returnvalue) _hp))))
        (:`then_1`
          (`KismetSystemLibrary.Delay` 0.5)
          (set `self.Taking Damage` false))))
    (:`then_8`
      (bind _aswater_beam (cast `/Game/Blueprints/Spells/Water/WaterBeam` OtherActor))
      (set `self.Taking Damage` true)
      (`|ExecutionSequence`
        (:`then_0`
          (if (`self.Passive 2`)
            (set `self.HP` (- (* (`/Game/Blueprints/Spells/Water/WaterBeam.Damage` _aswater_beam) _returnvalue) _hp))))
        (:`then_1`
          (`KismetSystemLibrary.Delay` 0.5)
          (set `self.Taking Damage` false))))
    (:`then_9`
      (bind _asgust_wind_blast (cast `/Game/Blueprints/Spells/Air/GustWindBlast` OtherActor))
      (set `self.Taking Damage` true)
      (`|ExecutionSequence`
        (:`then_0`
          (if (`self.Passive 2`)
            (set `self.HP` (- (* (`/Game/Blueprints/Spells/Air/GustWindBlast.Damage` _asgust_wind_blast) _returnvalue) _hp))))
        (:`then_1`
          (`KismetSystemLibrary.Delay` 0.5)
          (set `self.Taking Damage` false))))
    (:`then_10`
      (bind _asair_blast (cast `/Game/Blueprints/Spells/Air/AirBlast` OtherActor))
      (set `self.Taking Damage` true)
      (`|ExecutionSequence`
        (:`then_0`
          (if (`self.Passive 2`)
            (set `self.HP` (- (* (`/Game/Blueprints/Spells/Air/AirBlast.Damage` _asair_blast) _returnvalue) _hp))))
        (:`then_1`
          (`KismetSystemLibrary.Delay` 0.5)
          (set `self.Taking Damage` false))))
    (:`then_11`
      (bind _aswhirlwind (cast `/Game/Blueprints/Spells/Air/Whirlwind` OtherActor))
      (set `self.Taking Damage` true)
      (`|ExecutionSequence`
        (:`then_0`
          (if (`self.Passive 2`)
            (set `self.HP` (- (* (`/Game/Blueprints/Spells/Air/Whirlwind.Damage` _aswhirlwind) _returnvalue) _hp))))
        (:`then_1`
          (`KismetSystemLibrary.Delay` 0.5)
          (set `self.Taking Damage` false))))))

(fn `UserConstructionScript`)