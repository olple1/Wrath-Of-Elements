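; Fire golem enemy that wakes when the player gets close, then repeatedly fires from two attack boxes that track the player while InRange.
; Capsule overlaps identify each spell by cast; fire spells apply burn, with player passives controlling stacking, direct-hit damage and water slow.
; Tick updates HP text, burn damage and stack decay.
; On death it drops a random item, grants general and selected-element EXP, and may spawn a passive explosion.
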(event `self.ReceiveBeginPlay`
  (bind _character (`self.Character`))
  (bind _returnvalue (`KismetTextLibrary.Conv_DoubleToText` (`self.HP`) "HalfToEven"))
  (bind _returnvalue_2 (`GameplayStatics.LoadGameFromSlot` "Spell_Selection"))
  (bind _output_get (set `self.Save Game` _returnvalue_2))
  (bind _asspell_selection (cast `/Game/Blueprints/Spell_Selection` _output_get))
  (set `self.Fire Selected` (`/Game/Blueprints/Spell_Selection.Fire Element Selected` _asspell_selection))
  (set `self.Air Selected` (`/Game/Blueprints/Spell_Selection.Air Element Selected` _asspell_selection))
  (set `self.Water Selected` (`/Game/Blueprints/Spell_Selection.Water Element Selected` _asspell_selection))
  (set `self.Earth Selected` (`/Game/Blueprints/Spell_Selection.Earth Element Selected` _asspell_selection))
  (bind _asthird_person_character (cast `/Game/Blueprints/ThirdPersonBP/Blueprints/ThirdPersonCharacter` (`GameplayStatics.GetPlayerCharacter` 0)))
  (set `self.Character` _asthird_person_character)
  (set `self.Passive 2` (`/Game/Blueprints/ThirdPersonBP/Blueprints/ThirdPersonCharacter.Fire Passive 2` _character))
  (set `self.Passive 3` (`/Game/Blueprints/ThirdPersonBP/Blueprints/ThirdPersonCharacter.Fire Passive 3` _character))
  (set `self.Passive 4` (`/Game/Blueprints/ThirdPersonBP/Blueprints/ThirdPersonCharacter.Fire Passive 4` _character))
  (`TextRenderComponent.K2_SetText` (`self.Max hp`) _returnvalue)
  (`TextRenderComponent.K2_SetText` (`self.Current hp`) _returnvalue)
  (set `self.Speed` (`CharacterMovementComponent.MaxWalkSpeed` (`self.CharacterMovement`))))

(event `self.ReceiveTick`
  (params (DeltaSeconds :type "Float (single-precision)"))
  (bind (_returnvalue_x _returnvalue_y _returnvalue_z) (`KismetMathLibrary.BreakVector` (`self.K2_GetActorLocation`)))
  (bind _burn_count (`self.Burn Count`))
  (bind _exp (`self.EXP`))
  (bind _character (`self.Character`))
  (`|ExecutionSequence`
    (:`then_0`
      (`TextRenderComponent.K2_SetText` (`self.Current hp`) (`KismetTextLibrary.Conv_DoubleToText` (`self.HP`) "HalfToEven" false false 1 324 0 0))
      (if (<= (`self.HP`) 0.0)
        (`/Engine/EditorBlueprintResources/StandardMacros.DoOnce` false
          (:`Completed`
            (if (`self.Passive 4`)
              (if (>= (`self.Burn Count`) 4.0)
                (`|SpawnActorFromClass` "/Game/Blueprints/Spells/Fire/Passive_Explosion.Passive_Explosion_C" (`KismetMathLibrary.Conv_VectorToTransform` (`self.K2_GetActorLocation`)) "AlwaysSpawn" "OverrideRootScale" null null)))
            (switch `int` (`KismetMathLibrary.RandomIntegerInRange` 0 7)
              (:`0`
                (set `self.Item Dropped` "/Game/Blueprints/Items/Armor_item.Armor_item_C"))
              (:`1`
                (set `self.Item Dropped` "/Game/Blueprints/Items/Hp_item.Hp_item_C"))
              (:`2`
                (set `self.Item Dropped` "/Game/Blueprints/Items/Hp_Regen_item.Hp_Regen_item_C"))
              (:`3`
                (set `self.Item Dropped` "/Game/Blueprints/Items/Mana_item.Mana_item_C"))
              (:`4`
                (set `self.Item Dropped` "/Game/Blueprints/Items/Mana_Regen_item.Mana_Regen_item_C"))
              (:`5`
                (set `self.Item Dropped` "/Game/Blueprints/Items/Magic_power_item.Magic_Power_item_C"))
              (:`6`
                (set `self.Item Dropped` "/Game/Blueprints/Items/Movement_Speed_item.Movement_Speed_item_C"))
              (:`7`
                (set `self.Item Dropped` "/Game/Blueprints/Items/Cooldown_item.Cooldown_item_C"))
              (:`8`
                (set `self.Item Dropped` "/Game/Blueprints/Items/Crit_Damage_item.Crit_Damage_item_C")))
            (`/Engine/EditorBlueprintResources/StandardMacros.CompareInt` (`KismetMathLibrary.RandomIntegerInRange` 1 4) 3
              (:`>`
                _)
              (:`==`
                _)
              (:`<`
                _))
            (`|SpawnActorFromClass` (`self.Item Dropped`) (`KismetMathLibrary.MakeTransform` (`KismetMathLibrary.MakeVector` _returnvalue_x _returnvalue_y (- _returnvalue_z 400.0))) "AlwaysSpawn" "OverrideRootScale" null null)
            ;[1 1 1] EXP
            (set `/Game/Blueprints/ThirdPersonBP/Blueprints/ThirdPersonCharacter.EXP` (+ (`/Game/Blueprints/ThirdPersonBP/Blueprints/ThirdPersonCharacter.EXP` _character) _exp) _character)
            (`|ExecutionSequence`
              (:`then_0`
                (if (`self.Fire Selected`)
                  (set `/Game/Blueprints/ThirdPersonBP/Blueprints/ThirdPersonCharacter.Fire Magic EXP ` (+ (`/Game/Blueprints/ThirdPersonBP/Blueprints/ThirdPersonCharacter.Fire Magic EXP ` _character) _exp) _character)
                  (`self.K2_DestroyActor` :!label _label)))
              (:`then_1`
                (if (`self.Air Selected`)
                  (set `/Game/Blueprints/ThirdPersonBP/Blueprints/ThirdPersonCharacter.Air Magic EXP` (+ (`/Game/Blueprints/ThirdPersonBP/Blueprints/ThirdPersonCharacter.Air Magic EXP` _character) _exp) _character)
                  (goto _label)))
              (:`then_2`
                (if (`self.Water Selected`)
                  (set `/Game/Blueprints/ThirdPersonBP/Blueprints/ThirdPersonCharacter.Water Magic EXP` (+ (`/Game/Blueprints/ThirdPersonBP/Blueprints/ThirdPersonCharacter.Water Magic EXP` _character) _exp) _character)
                  (goto _label)))
              (:`then_3`
                (if (`self.Earth Selected`)
                  (set `/Game/Blueprints/ThirdPersonBP/Blueprints/ThirdPersonCharacter.Earth Magic EXP` (+ (`/Game/Blueprints/ThirdPersonBP/Blueprints/ThirdPersonCharacter.Earth Magic EXP` _character) _exp) _character)
                  (goto _label))))))))
    (:`then_1`
      (set `self.DeltaTime` DeltaSeconds)
      (`self.ProjectileRotation`))
    (:`then_2`
      (`KismetSystemLibrary.Delay` 1.0)
      (if (`self.Burning`)
        (set `self.HP` (- (`self.HP`) (`self.Burn Damage`)))))
    (:`then_3`
      (if (`self.Passive 3`)
        (`KismetSystemLibrary.Delay` 2.0)
        (set `self.Burn Count` (- _burn_count 1.0))
        (if (>= 0.0 _burn_count)
          (set `self.Burning` false))))))

(event `self.Player Close.OnComponentBeginOverlap`
  (params (OverlappedComponent :type "PrimitiveComponent Object Reference") (OtherActor :type "Actor Object Reference") (OtherComp :type "PrimitiveComponent Object Reference") (OtherBodyIndex :type Integer) (bFromSweep :type Boolean) (SweepResult :type "HitResult Structure (by ref)"))
  (cast `/Game/Blueprints/ThirdPersonBP/Blueprints/ThirdPersonCharacter` OtherActor)
  (`self.Voke Golem`)
  (`KismetSystemLibrary.Delay` 6.0)
  (`self.ShootAtPlayer`)
  (`self.Attack`))

(event `Attack`
  ;[1 1 1] Animation
  (set `self.Attacking` true))

(event `Voke Golem`
  ;[1 1 1] Animation
  (`/Engine/EditorBlueprintResources/StandardMacros.DoOnce` false
    (:`Completed`
      (set `self.Voke` true)
      (set `self.Sleep` false))))

(event `self.CapsuleComponent.OnComponentBeginOverlap`
  (params (OverlappedComponent :type "PrimitiveComponent Object Reference") (OtherActor :type "Actor Object Reference") (OtherComp :type "PrimitiveComponent Object Reference") (OtherBodyIndex :type Integer) (bFromSweep :type Boolean) (SweepResult :type "HitResult Structure (by ref)"))
  (bind _passive_3 (`self.Passive 3`))
  (bind _passive_3_2 (`self.Passive 3`))
  (bind _passive_3_3 (`self.Passive 3`))
  (bind _charactermovement (`self.CharacterMovement`))
  (bind _returnvalue (* (`self.Burn Count`) 0.1))
  ;[1 1 1] Burn Damage
  (`|ExecutionSequence`
    (:`then_0`
      (bind _asfireball (cast `/Game/Blueprints/Spells/Fire/Fireball` OtherActor))
      (set `self.Taking Damage` true)
      (`|ExecutionSequence`
        (:`then_0`
          (`/Engine/EditorBlueprintResources/StandardMacros.CompareFloat` (`self.Burn Count`) 1.0
            (:`>`
              (if _passive_3
                (if _passive_3 :!label _label_2
                  (set `self.Burn Count` (+ (`self.Burn Count`) 1.0))
                  (else
                    (set `self.Burn Count` 1.0)))
                (set `self.Burn Damage` (* (* (`/Game/Blueprints/Spells/Fire/Fireball.Damage` _asfireball) 0.02) (`self.Burn Count`)))))
            (:`==`
              (set `self.Strongest burn` 1.0 :!label _label_3)
              (goto _label_2))
            (:`<`
              (goto _label_3)))
          (`self.K2_DestroyActor` _asfireball)
          (set `self.Burning` true)
          (`KismetSystemLibrary.Delay` 3.0)
          (if (not (`self.Passive 3`))
            (if (>= (`self.Burn Count`) (`self.Strongest burn`)) :!label _label_4
              (set `self.Burning` false :!label _label_5)
              (set `self.Burn Count` 0.0)
              (set `self.Strongest burn` 0.0))))
        (:`then_1`
          (if (`self.Passive 2`)
            (bind _damage (`/Game/Blueprints/Spells/Fire/Fireball.Damage` _asfireball))
            (set `self.HP` (- (`self.HP`) (+ (* _damage _returnvalue) _damage)))))
        (:`then_2`
          (`KismetSystemLibrary.Delay` 0.5)
          (set `self.Taking Damage` false))))
    (:`then_1`
      (bind _asfire_wall (cast `/Game/Blueprints/Spells/Fire/FireWall` OtherActor))
      (set `self.Taking Damage` true)
      (`|ExecutionSequence`
        (:`then_0`
          (`/Engine/EditorBlueprintResources/StandardMacros.CompareFloat` (`self.Burn Count`) 2.0
            (:`>`
              (if _passive_3_2
                (if _passive_3_2 :!label _label_6
                  (set `self.Burn Count` (+ (`self.Burn Count`) 2.0))
                  (else
                    (set `self.Burn Count` 2.0)))
                (set `self.Burn Damage` (* (* (`/Game/Blueprints/Spells/Fire/FireWall.Damage` _asfire_wall) 0.02) (`self.Burn Count`)))
                (set `self.Burning` true)
                (`KismetSystemLibrary.Delay` 5.0)
                (if (not (`self.Passive 3`))
                  (goto _label_4))))
            (:`==`
              (set `self.Strongest burn` 2.0 :!label _label_7)
              (goto _label_6))
            (:`<`
              (goto _label_7))))
        (:`then_1`
          (if (`self.Passive 2`)
            (bind _damage_2 (`/Game/Blueprints/Spells/Fire/FireWall.Damage` _asfire_wall))
            (set `self.HP` (- (`self.HP`) (+ (* _damage_2 _returnvalue) _damage_2)))))
        (:`then_2`
          (`KismetSystemLibrary.Delay` 0.5)
          (set `self.Taking Damage` false))))
    (:`then_2`
      (bind _asflame_strike (cast `/Game/Blueprints/Spells/Fire/Flame_Strike` OtherActor))
      (set `self.Taking Damage` true)
      (`|ExecutionSequence`
        (:`then_0`
          (`/Engine/EditorBlueprintResources/StandardMacros.CompareFloat` (`self.Burn Count`) 3.0
            (:`>`
              (if _passive_3_3
                (if _passive_3_3 :!label _label_8
                  (set `self.Burn Count` (+ (`self.Burn Count`) 3.0))
                  (else
                    (set `self.Burn Count` 3.0)))
                (set `self.Burn Damage` (* (* (`/Game/Blueprints/Spells/Fire/Flame_Strike.Damage` _asflame_strike) 0.02) (`self.Burn Count`)))
                (set `self.Burning` true)
                (`KismetSystemLibrary.Delay` 7.0)
                (if (not (`self.Passive 3`))
                  (goto _label_4))))
            (:`==`
              (set `self.Strongest burn` 3.0 :!label _label_9)
              (goto _label_8))
            (:`<`
              (goto _label_9))))
        (:`then_1`
          (if (`self.Passive 2`)
            (bind _damage_3 (`/Game/Blueprints/Spells/Fire/Flame_Strike.Damage` _asflame_strike))
            (set `self.HP` (- (`self.HP`) (+ (* _damage_3 _returnvalue) _damage_3)))))
        (:`then_2`
          (`KismetSystemLibrary.Delay` 0.5)
          (set `self.Taking Damage` false))))
    (:`then_3`
      (bind _asmeteor (cast `/Game/Blueprints/Spells/Fire/Meteor` OtherActor))
      (set `self.Taking Damage` true)
      (`|ExecutionSequence`
        (:`then_0`
          (set `self.Strongest burn` 4.0)
          (if (`self.Passive 3`)
            (set `self.Burn Count` (+ (`self.Burn Count`) 4.0))
            (else
              (set `self.Burn Count` 4.0)))
          (set `self.Burn Damage` (* (* (`/Game/Blueprints/Spells/Fire/Meteor.Damage` _asmeteor) 0.02) (`self.Burn Count`)))
          (set `self.Burning` true)
          (`KismetSystemLibrary.Delay` 10.0)
          (if (not (`self.Passive 3`))
            (goto _label_5)))
        (:`then_1`
          (if (`self.Passive 2`)
            (bind _damage_4 (`/Game/Blueprints/Spells/Fire/Meteor.Damage` _asmeteor))
            (set `self.HP` (- (`self.HP`) (+ (* _damage_4 _returnvalue) _damage_4)))))
        (:`then_2`
          (`KismetSystemLibrary.Delay` 0.5)
          (set `self.Taking Damage` false))))
    (:`then_4`
      (bind _asearthquake (cast `/Game/Blueprints/Spells/Earth/Earthquake` OtherActor))
      (set `self.Taking Damage` true)
      (`|ExecutionSequence`
        (:`then_0`
          (if (`self.Passive 2`)
            (bind _damage_5 (`/Game/Blueprints/Spells/Earth/Earthquake.Damage` _asearthquake))
            (set `self.HP` (- (`self.HP`) (+ (* _damage_5 _returnvalue) _damage_5)))))
        (:`then_1`
          (`KismetSystemLibrary.Delay` 0.5)
          (set `self.Taking Damage` false))))
    (:`then_5`
      (bind _asrock_blast (cast `/Game/Blueprints/Spells/Earth/RockBlast` OtherActor))
      (set `self.Taking Damage` true)
      (`|ExecutionSequence`
        (:`then_0`
          (if (`self.Passive 2`)
            (bind _damage_6 (`/Game/Blueprints/Spells/Earth/RockBlast.Damage` _asrock_blast))
            (set `self.HP` (- (`self.HP`) (+ (* _damage_6 _returnvalue) _damage_6)))))
        (:`then_1`
          (`KismetSystemLibrary.Delay` 0.5)
          (set `self.Taking Damage` false))))
    (:`then_6`
      (bind _asaftershock (cast `/Game/Blueprints/Spells/Earth/Aftershock` OtherActor))
      (set `self.Taking Damage` true)
      (`|ExecutionSequence`
        (:`then_0`
          (if (`self.Passive 2`)
            (bind _damage_7 (`/Game/Blueprints/Spells/Earth/Aftershock.Damage` _asaftershock))
            (set `self.HP` (- (`self.HP`) (+ (* _damage_7 _returnvalue) _damage_7)))))
        (:`then_1`
          (`KismetSystemLibrary.Delay` 0.5)
          (set `self.Taking Damage` false))))
    (:`then_7`
      (bind _aswater_bolt (cast `/Game/Blueprints/Spells/Water/WaterBolt` OtherActor))
      (set `self.Taking Damage` true)
      (`|ExecutionSequence`
        (:`then_0`
          (if (`self.Passive 2`)
            (bind _damage_8 (`/Game/Blueprints/Spells/Water/WaterBolt.Damage` _aswater_bolt))
            (set `self.HP` (- (`self.HP`) (+ (* _damage_8 _returnvalue) _damage_8)))))
        (:`then_1`
          (`KismetSystemLibrary.Delay` 0.5)
          (set `self.Taking Damage` false)
          (if (`/Game/Blueprints/ThirdPersonBP/Blueprints/ThirdPersonCharacter.Water Passive 4` (`self.Character`)) :!label _label_10
            (set `CharacterMovementComponent.MaxWalkSpeed` (/ (`CharacterMovementComponent.MaxWalkSpeed` _charactermovement) 1.2) _charactermovement)
            (`KismetSystemLibrary.RetriggerableDelay` 3.0)))))
    (:`then_8`
      (bind _aswater_beam (cast `/Game/Blueprints/Spells/Water/WaterBeam` OtherActor))
      (set `self.Taking Damage` true)
      (`|ExecutionSequence`
        (:`then_0`
          (if (`self.Passive 2`)
            (bind _damage_9 (`/Game/Blueprints/Spells/Water/WaterBeam.Damage` _aswater_beam))
            (set `self.HP` (- (`self.HP`) (+ (* _damage_9 _returnvalue) _damage_9)))))
        (:`then_1`
          (`KismetSystemLibrary.Delay` 0.5)
          (set `self.Taking Damage` false)
          (goto _label_10))))
    (:`then_9`
      (bind _asgust_wind_blast (cast `/Game/Blueprints/Spells/Air/GustWindBlast` OtherActor))
      (set `self.Taking Damage` true)
      (`|ExecutionSequence`
        (:`then_0`
          (if (`self.Passive 2`)
            (bind _damage_10 (`/Game/Blueprints/Spells/Air/GustWindBlast.Damage` _asgust_wind_blast))
            (set `self.HP` (- (`self.HP`) (+ (* _damage_10 _returnvalue) _damage_10)))))
        (:`then_1`
          (`KismetSystemLibrary.Delay` 0.5)
          (set `self.Taking Damage` false))))
    (:`then_10`
      (bind _asair_blast (cast `/Game/Blueprints/Spells/Air/AirBlast` OtherActor))
      (set `self.Taking Damage` true)
      (`|ExecutionSequence`
        (:`then_0`
          (if (`self.Passive 2`)
            (bind _damage_11 (`/Game/Blueprints/Spells/Air/AirBlast.Damage` _asair_blast))
            (set `self.HP` (- (`self.HP`) (+ (* _damage_11 _returnvalue) _damage_11)))))
        (:`then_1`
          (`KismetSystemLibrary.Delay` 0.5)
          (set `self.Taking Damage` false))))
    (:`then_11`
      (bind _aswhirlwind (cast `/Game/Blueprints/Spells/Air/Whirlwind` OtherActor))
      (set `self.Taking Damage` true)
      (`|ExecutionSequence`
        (:`then_0`
          (if (`self.Passive 2`)
            (bind _damage_12 (`/Game/Blueprints/Spells/Air/Whirlwind.Damage` _aswhirlwind))
            (set `self.HP` (- (`self.HP`) (+ (* _damage_12 _returnvalue) _damage_12)))))
        (:`then_1`
          (`KismetSystemLibrary.Delay` 0.5)
          (set `self.Taking Damage` false))))))

(event `ShootAtPlayer`
  ;[1 1 1] Shoots at the Player
  (`|SpawnActorFromClass` "/Game/Enemies/ElementalGolems/FireGolem/FireGolem_attack.FireGolem_attack_C" (`SceneComponent.GetSocketTransform` (`self.Attack box 2`) "None" "RTS_World") "AlwaysSpawn" "OverrideRootScale" null null)
  (`KismetSystemLibrary.Delay` 0.4)
  (`|SpawnActorFromClass` "/Game/Enemies/ElementalGolems/FireGolem/FireGolem_attack.FireGolem_attack_C" (`SceneComponent.GetSocketTransform` (`self.Attack box 1`) "None" "RTS_World") "AlwaysSpawn" "OverrideRootScale" null null)
  (`GameplayStatics.SpawnSoundAtLocation` null (`self.K2_GetActorLocation`) (struct) 1.0 1.0 0.0 null null)
  (`KismetSystemLibrary.RetriggerableDelay` (`self.FireRate`))
  (`self.ShootAtPlayer`))

(event `ProjectileRotation`
  (bind _attack_box_1 (`self.Attack box 1`))
  (bind _attack_box_2 (`self.Attack box 2`))
  ;[1 1 1] Projectile Rotation
  (if (`self.InRange`)
    (`|ExecutionSequence`
      (:`then_0`
        (`SceneComponent.K2_SetWorldRotation` _attack_box_1 (`KismetMathLibrary.RInterpTo` (`SceneComponent.K2_GetComponentRotation` _attack_box_1) (`KismetMathLibrary.MakeRotator` 0.0 (.pitch (`KismetMathLibrary.FindLookAtRotation` (`SceneComponent.K2_GetComponentLocation` (`self.Attack box 1`)) (`self.K2_GetActorLocation` (`GameplayStatics.GetPlayerCharacter` 0)))) (.yaw (`KismetMathLibrary.FindLookAtRotation` (`SceneComponent.K2_GetComponentLocation` (`self.Attack box 1`)) (`self.K2_GetActorLocation` (`GameplayStatics.GetPlayerCharacter` 0))))) (`self.DeltaTime`) (`self.RotationSpeed`)) false false))
      (:`then_1`
        (`SceneComponent.K2_SetWorldRotation` _attack_box_2 (`KismetMathLibrary.RInterpTo` (`SceneComponent.K2_GetComponentRotation` _attack_box_2) (`KismetMathLibrary.MakeRotator` 0.0 (.pitch (`KismetMathLibrary.FindLookAtRotation` (`SceneComponent.K2_GetComponentLocation` (`self.Attack box 2`)) (`self.K2_GetActorLocation` (`GameplayStatics.GetPlayerCharacter` 0)))) (.yaw (`KismetMathLibrary.FindLookAtRotation` (`SceneComponent.K2_GetComponentLocation` (`self.Attack box 2`)) (`self.K2_GetActorLocation` (`GameplayStatics.GetPlayerCharacter` 0))))) (`self.DeltaTime`) (`self.RotationSpeed`)) false false)))))

(fn `UserConstructionScript`)